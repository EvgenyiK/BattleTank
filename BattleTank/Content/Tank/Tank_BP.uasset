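; Tank Blueprint for a player-controllable tank with camera aiming and firing.
; On BeginPlay it passes the Barrel and Turret components to SetBarrelReference and SetTurretReference.
; Aim axes rotate the AzimutGimbal in yaw and the SpringArm in pitch, scaled by frame delta time, separating the two rotations.
; The Fire input calls the Fire function, whose logic is defined outside these graphs.
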(event EventBeginPlay
  (Class|Tank|SetBarrelReference (Variables|Components|GetBarrel))
  (Class|Tank|SetTurretReference (Variables|Default|GetTurret)))

(event Input|ActionEvents|InputActionFire
  (params (Key :type Key%20Structure :default "None"))
  ;[1 1 1] input binding
  (:Pressed
    (Class|Tank|Fire)))

(event Input|AxisEvents|InputAxisAimAzimut
  (params (AxisValue :type Float%20%28single-precision%29))
  ;[1 1 1] input binding
  (Transformation|AddLocalRotation (Variables|Components|GetAzimut%20Gimbal) (Math|Rotator|MakeRotator 0.0 0.0 (* AxisValue (Utilities|Time|GetWorldDeltaSeconds) 1e+02)) false false))

(event Input|AxisEvents|InputAxisAimElevation
  (params (AxisValue :type Float%20%28single-precision%29))
  ;[1 1 1] input binding
  (Transformation|AddLocalRotation (Variables|Components|GetSpringArm) (Math|Rotator|MakeRotator 0.0 (* AxisValue (Utilities|Time|GetWorldDeltaSeconds) 1e+02) 0.0) false false))

(fn ConstructionScript)